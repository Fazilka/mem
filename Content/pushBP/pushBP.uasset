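; Pushable block actor that the player character (characterBP) can move by walking into it.
; Overlapping either the X-axis or Y-axis trigger turns on physics simulation for the Cube and sets the character's IsPushing flag.
; Leaving either trigger reverses both, regardless of whether the character still overlaps the other one.
; Both triggers run identical logic, with no axis constraint applied in the graph.
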(event OnComponentBeginOverlap(YAxisCol)
  (params (OverlappedComponent :type Primitive%20Component%20Object%20Reference) (OtherActor :type Actor%20Object%20Reference) (OtherComp :type Primitive%20Component%20Object%20Reference) (OtherBodyIndex :type Integer) (bFromSweep :type Boolean) (SweepResult :type Hit%20Result%20Structure%20%28by%20ref%29))
  ;[1 1 1] Y AX COL PUSH
  (bind _ascharacter_bp (Utilities|Casting|CastTocharacterBP OtherActor))
  (Physics|SetSimulatePhysics (Variables|Default|GetCube) true)
  (Variables|/Game/characterBP.characterBP_C|SetIsPushing? _ascharacter_bp true))

(event OnComponentEndOverlap(YAxisCol)
  (params (OverlappedComponent :type Primitive%20Component%20Object%20Reference) (OtherActor :type Actor%20Object%20Reference) (OtherComp :type Primitive%20Component%20Object%20Reference) (OtherBodyIndex :type Integer))
  ;[1 1 1] Y AX COL PUSH
  (bind _ascharacter_bp (Utilities|Casting|CastTocharacterBP OtherActor))
  (Physics|SetSimulatePhysics (Variables|Default|GetCube) false)
  (Variables|/Game/characterBP.characterBP_C|SetIsPushing? _ascharacter_bp false))

(event OnComponentBeginOverlap(XAxisCol)
  (params (OverlappedComponent :type Primitive%20Component%20Object%20Reference) (OtherActor :type Actor%20Object%20Reference) (OtherComp :type Primitive%20Component%20Object%20Reference) (OtherBodyIndex :type Integer) (bFromSweep :type Boolean) (SweepResult :type Hit%20Result%20Structure%20%28by%20ref%29))
  ;[1 1 1] Y AX COL PUSH
  (bind _ascharacter_bp (Utilities|Casting|CastTocharacterBP OtherActor))
  (Physics|SetSimulatePhysics (Variables|Default|GetCube) true)
  (Variables|/Game/characterBP.characterBP_C|SetIsPushing? _ascharacter_bp true))

(event OnComponentEndOverlap(XAxisCol)
  (params (OverlappedComponent :type Primitive%20Component%20Object%20Reference) (OtherActor :type Actor%20Object%20Reference) (OtherComp :type Primitive%20Component%20Object%20Reference) (OtherBodyIndex :type Integer))
  ;[1 1 1] Y AX COL PUSH
  (bind _ascharacter_bp (Utilities|Casting|CastTocharacterBP OtherActor))
  (Physics|SetSimulatePhysics (Variables|Default|GetCube) false)
  (Variables|/Game/characterBP.characterBP_C|SetIsPushing? _ascharacter_bp false))

(event EventBeginPlay)

(event Collision|EventActorBeginOverlap
  (params (OtherActor :type Actor%20Object%20Reference)))

(event EventTick
  (params (DeltaSeconds :type Float%20%28single-precision%29)))

(fn ConstructionScript)